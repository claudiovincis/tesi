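; GameHUD creates the on-screen widgets and feeds them live player and boss state.
; On BeginPlay it caches the ThirdPersonCharacter_2 player and its Boss reference, then adds the HUD and HUD_VideoMenu widgets to the viewport.
; Every Tick it copies boss and player life, plus the player's Recognized and ObjectCatch states, into the HUD widget by polling rather than events.
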(event EventBeginPlay
  (bind _asthird_person_character_2 (Utilities|Casting|CastToThirdPersonCharacter_2 (Game|GetPlayerCharacter 0)))
  (Variables|Default|SetMC _asthird_person_character_2)
  (Variables|Default|SetBoss (Variables|/Game/ThirdPersonBP/Blueprints/ThirdPersonCharacter_2.ThirdPersonCharacter_2_C|GetBoss _asthird_person_character_2))
  (bind _returnvalue (UserInterface|CreateWidget "/Game/Components/HUD.HUD_C"))
  (bind _output_get (Variables|Default|SetHUD _returnvalue))
  (UserInterface|Viewport|AddtoViewport _output_get 0)
  (bind _returnvalue_2 (UserInterface|CreateWidget "/Game/Components/HUD_VideoMenu.HUD_VideoMenu_C"))
  (bind _output_get_2 (Variables|Default|SetHudVideoMenu _returnvalue_2))
  (UserInterface|Viewport|AddtoViewport _output_get_2 0))

(event Collision|EventActorBeginOverlap
  (params (OtherActor :type Actor%20Object%20Reference)))

(event EventTick
  (params (DeltaSeconds :type Float%20%28single-precision%29))
  (bind _hud (Variables|Default|GetHUD))
  (bind _mc (Variables|Default|GetMC))
  (bind _hud_2 (Variables|Default|GetHUD))
  (Variables|/Game/Components/HUD.HUD_C|SetHealthBoss _hud_2 (Math|Conversions|ToFloat(Integer) (Variables|/Game/Components/Boss.Boss_C|GetLife (Variables|Default|GetBoss))))
  (Variables|/Game/Components/HUD.HUD_C|SetHealthMC _hud_2 (Math|Conversions|ToFloat(Integer) (Variables|/Game/ThirdPersonBP/Blueprints/ThirdPersonCharacter_2.ThirdPersonCharacter_2_C|GetLife (Variables|Default|GetMC))))
  (Variables|/Game/Components/HUD.HUD_C|SetRecognized _hud (Variables|/Game/ThirdPersonBP/Blueprints/ThirdPersonCharacter_2.ThirdPersonCharacter_2_C|GetRecognized _mc))
  (Variables|/Game/Components/HUD.HUD_C|SetObjectCatch _hud (Variables|/Game/ThirdPersonBP/Blueprints/ThirdPersonCharacter_2.ThirdPersonCharacter_2_C|GetObjectCatch _mc)))

(fn ConstructionScript)