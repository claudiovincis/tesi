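; FloatingProps is an actor component that makes its owning prop float by animating its location and rotation in a loop.
; BeginPlay caches the owner's starting transform as the base.
; Each Tick advances separate position and rotation timers, scaled by their frequency multipliers and wrapped to 0–1.
; MoveEvent samples a shared float curve at those times to scale configurable offsets, which it applies to the base without sweeping.
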(event Custom|MoveEvent
  (bind _returnvalue (Components|GetOwner))
  (Transformation|SetActorLocation _returnvalue (+ (Variables|Default|GetActorInitialLocation) (* (Variables|Default|GetPositionRangeAdder) (Math|Curves|GetFloatValue (Variables|Default|GetCurveToUse) (Variables|Default|GetTimeElapsedPosition)))) false false)
  (Transformation|SetActorRotation _returnvalue (Math|Rotator|CombineRotators (Variables|Default|GetActorInitialRotation) (* (Variables|Default|GetRotationRangeAdder) (Math|Curves|GetFloatValue (Variables|Default|GetCurveToUse) (Variables|Default|GetTimeElapsedRotation))))))

(event EventBeginPlay
  (bind _returnvalue (Components|GetOwner))
  (Variables|Default|SetActorInitialLocation (Transformation|GetActorLocation _returnvalue))
  (Variables|Default|SetActorInitialRotation (Transformation|GetActorRotation _returnvalue)))

(event EventTick
  (params (DeltaSeconds :type Float%20%28single-precision%29))
  (Variables|Default|SetTimeElapsedPosition (Math|Float|%(Float) (+ (Variables|Default|GetTimeElapsedPosition) (/ DeltaSeconds (/ 1.0 (Variables|Default|GetFrequencyPositionMultiplier)))) 1.0))
  (Variables|Default|SetTimeElapsedRotation (Math|Float|%(Float) (+ (Variables|Default|GetTimeElapsedRotation) (/ DeltaSeconds (/ 1.0 (Variables|Default|GetFrequencyRotationMultiplier)))) 1.0))
  (CallFunction|MoveEvent))